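; Player character for a card-based puzzle game that turns keyboard presses into card manager commands.
; On BeginPlay it finds and stores the level's BP_CardManager.
; Space requests a new hand of cards and spawns them after a short delay, Backspace triggers the manager's choose-card event, and Escape quits the game.
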(event `self.ReceiveBeginPlay`
  ;[1 1 1] Begin Play
  (bind _outactors (`GameplayStatics.GetAllActorsOfClass` "/Game/Blueprints/BP_CardManager.BP_CardManager_C"))
  (set `self.BP_CardManager` (`|GetArrayItem` _outactors)))

(event `Key|SpaceBar`
  (params (Key :type "Key Structure"))
  (bind _bp_cardmanager (`self.BP_CardManager`))
  ;[1 1 1] New Cards
  (:`Pressed`
    (`/Game/Blueprints/BP_CardManager.Event NewHandOfCards` _bp_cardmanager)
    (`KismetSystemLibrary.Delay` 0.2)
    (`/Game/Blueprints/BP_CardManager.Event SpawnCards` _bp_cardmanager)))

(event `Key|BackSpace`
  (params (Key :type "Key Structure"))
  (:`Pressed`
    (`/Game/Blueprints/BP_CardManager.Event ChooseCard` (`self.BP_CardManager`))))

(event `Key|Escape`
  (params (Key :type "Key Structure"))
  (:`Pressed`
    (`KismetSystemLibrary.QuitGame` null "Quit")))

(fn `UserConstructionScript`)