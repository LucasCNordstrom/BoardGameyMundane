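; BP_PutOnMusic is an effect actor, apparently for a card, that trades player health for a bonus to the next task.
; On BeginPlay it raises BP_TaskManager's NextTaskModifier, lowers BP_CardManager's PlayerHP, then refreshes the first WBP_GUI widget.
; The current-deck GUI update and DestroyActor nodes are unconnected, so the actor does not destroy itself.
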(event `self.ReceiveBeginPlay`
  (bind _returnvalue (`GameplayStatics.GetActorOfClass` "/Game/Blueprints/BP_TaskManager.BP_TaskManager_C"))
  (set `/Game/Blueprints/BP_TaskManager.NextTaskModifier` (+ (`/Game/Blueprints/BP_TaskManager.NextTaskModifier` _returnvalue) 3) _returnvalue)
  (bind _returnvalue_2 (`GameplayStatics.GetActorOfClass` "/Game/Blueprints/BP_CardManager.BP_CardManager_C"))
  (set `/Game/Blueprints/BP_CardManager.PlayerHP` (- (`/Game/Blueprints/BP_CardManager.PlayerHP` _returnvalue_2) 1) _returnvalue_2)
  (bind _foundwidgets (`WidgetBlueprintLibrary.GetAllWidgetsOfClass` "/Game/Blueprints/WBP_GUI.WBP_GUI_C"))
  (`/Game/Blueprints/WBP_GUI.Event UpdateGUI` (`|GetArrayItem` _foundwidgets))
  (`GameplayStatics.GetActorOfClass` "/Game/Blueprints/BP_CardManager.BP_CardManager_C"))

(fn `UserConstructionScript`)