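; Blueprint function library that fills the GUI tooltip text for cards and tasks in a card game about completing household chores.
; One function switches on card type and the other on task type, each writing to the GUI's TextBlockTooltip.
; Names come from the enum values, while effects, time costs, task values and completion rewards are hardcoded in each case's format string.
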(fn `FL_CardTooltip`
  (params (CardType :type "/Game/E_CardTypes Enum" :default "NewEnumerator0") (GUI :type "/Game/Blueprints/WBP_GUI Object Reference"))
  (bind _textblock_tooltip (`/Game/Blueprints/WBP_GUI.TextBlock_Tooltip` GUI))
  (switch `/Game/E_CardTypes` CardType
    (:`NewEnumerator0`
      (`TextBlock.SetText` _textblock_tooltip (`|FormatText` "Card: {CardName} \n---------------------- \nReduce Task by 2 \nCosts 5 time" (`KismetTextLibrary.Conv_StringToText` (`|GetEnumeratorNameAsString` CardType)))))
    (:`NewEnumerator1`
      (`TextBlock.SetText` _textblock_tooltip (`|FormatText` "Card: {CardName} \n---------------------- \nReduce Task by 3 \nCosts 10 time" (`KismetTextLibrary.Conv_StringToText` (`|GetEnumeratorNameAsString` CardType)))))
    (:`NewEnumerator2`
      (`TextBlock.SetText` _textblock_tooltip (`|FormatText` "Card: {CardName} \n---------------------- \nDraw 3 cards  \nCosts 10 time" (`KismetTextLibrary.Conv_StringToText` (`|GetEnumeratorNameAsString` CardType)))))
    (:`NewEnumerator5`
      (`TextBlock.SetText` _textblock_tooltip (`|FormatText` "Card: {CardName} \n---------------------- \nDraw 3 cards \nAdd a Bad tummy \nto deck \nCosts 5 time" (`KismetTextLibrary.Conv_StringToText` (`|GetEnumeratorNameAsString` CardType)))))
    (:`NewEnumerator6`
      (`TextBlock.SetText` _textblock_tooltip (`|FormatText` "Card: {CardName} \n---------------------- \nReduce Task by 4 \nCosts 10 time" (`KismetTextLibrary.Conv_StringToText` (`|GetEnumeratorNameAsString` CardType)))))
    (:`NewEnumerator7`
      (`TextBlock.SetText` _textblock_tooltip (`|FormatText` "Card: {CardName} \n---------------------- \nReduce next Task \nwith 3 \nCosts 20 time" (`KismetTextLibrary.Conv_StringToText` (`|GetEnumeratorNameAsString` CardType)))))
    (:`NewEnumerator8`
      (`TextBlock.SetText` _textblock_tooltip (`|FormatText` "Card: {CardName} \n---------------------- \nDiscards a  \nrandom card" (`KismetTextLibrary.Conv_StringToText` (`|GetEnumeratorNameAsString` CardType)))))))

(fn `FL_TaskTooltip`
  (params (TaskType :type "/Game/E_TaskTypes Enum" :default "NewEnumerator0") (GUI :type "/Game/Blueprints/WBP_GUI Object Reference"))
  (bind _textblock_tooltip (`/Game/Blueprints/WBP_GUI.TextBlock_Tooltip` GUI))
  (switch `/Game/E_TaskTypes` TaskType
    (:`NewEnumerator0`
      (`TextBlock.SetText` _textblock_tooltip (`|FormatText` "Task: {TaskName} \n---------------------- \nTask : 15" (`KismetTextLibrary.Conv_StringToText` (`|GetEnumeratorNameAsString` TaskType)))))
    (:`NewEnumerator1`
      (`TextBlock.SetText` _textblock_tooltip (`|FormatText` "Task: {TaskName} \n---------------------- \nTask : 13" (`KismetTextLibrary.Conv_StringToText` (`|GetEnumeratorNameAsString` TaskType)))))
    (:`NewEnumerator2`
      (`TextBlock.SetText` _textblock_tooltip (`|FormatText` "Task: {TaskName} \n---------------------- \nTask : 18 \nWhen finished: \nStart next task with 2 \nGet additional card " (`KismetTextLibrary.Conv_StringToText` (`|GetEnumeratorNameAsString` TaskType)))))
    (:`NewEnumerator4`
      (`TextBlock.SetText` _textblock_tooltip (`|FormatText` "Task: {TaskName} \n---------------------- \nTask : 12 \nWhen finished: \nGet additional card " (`KismetTextLibrary.Conv_StringToText` (`|GetEnumeratorNameAsString` TaskType)))))
    (:`NewEnumerator5`
      (`TextBlock.SetText` _textblock_tooltip (`|FormatText` "Task: {TaskName} \n---------------------- \nTask : 14" (`KismetTextLibrary.Conv_StringToText` (`|GetEnumeratorNameAsString` TaskType)))))
    (:`NewEnumerator6`
      (`TextBlock.SetText` _textblock_tooltip (`|FormatText` "Task: {TaskName} \n---------------------- \nTask : 15" (`KismetTextLibrary.Conv_StringToText` (`|GetEnumeratorNameAsString` TaskType)))))))