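; BP_TaskManager tracks the current chore in a card game, with each task type setting a target value.
; On BeginPlay it waits briefly, then caches the GUI widget and BP_CardManager.
; Choosing a task hides the selection arrow, applies any one-shot next-task modifier, refreshes the GUI and requests a new hand.
; Finishing a task has the card manager clear the table and start card choice; DoTask is an empty switch.
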(event `self.ReceiveBeginPlay`
  (`KismetSystemLibrary.Delay` 0.5)
  (bind _foundwidgets (`WidgetBlueprintLibrary.GetAllWidgetsOfClass` "/Game/Blueprints/WBP_GUI.WBP_GUI_C"))
  (set `self.GUI` (`|GetArrayItem` _foundwidgets))
  (bind _outactors (`GameplayStatics.GetAllActorsOfClass` "/Game/Blueprints/BP_CardManager.BP_CardManager_C"))
  (set `self.CardManager` (`|GetArrayItem` _outactors)))

(event `Event ChooseNewTask`
  (`SceneComponent.SetHiddenInGame` (`self.Arrow`) false true))

(event `Event SetCurrentTask`
  (params (ChooseTask :type "/Game/E_TaskTypes Enum" :default "NewEnumerator0"))
  (set `self.TaskType` ChooseTask)
  (`SceneComponent.SetHiddenInGame` (`self.Arrow`) true true)
  (switch `/Game/E_TaskTypes` (`self.TaskType`)
    (:`NewEnumerator0`
      (set `self.CurrentTaskValue` 11))
    (:`NewEnumerator1`
      (set `self.CurrentTaskValue` 8))
    (:`NewEnumerator2`
      (set `self.CurrentTaskValue` 5)))
  (if (`self.UseNextTaskModifier`)
    (set `self.CurrentTaskValue` (+ (`self.CurrentTaskValue`) (`self.NextTaskModifier`)))
    (set `self.UseNextTaskModifier` false))
  (`/Game/Blueprints/WBP_GUI.Event UpdateGUI` (`self.GUI`))
  (`/Game/Blueprints/BP_CardManager.Event NewHandOfCards` (`self.CardManager`)))

(event `Event TaskDone`
  (bind _cardmanager (`self.CardManager`))
  (`/Game/Blueprints/BP_CardManager.Event RemoveCardsOnTable` _cardmanager)
  (`/Game/Blueprints/BP_CardManager.Event ChooseCard` _cardmanager))

(event `Event DoTask`
  (switch `/Game/E_TaskTypes` (`self.TaskType`)))

(fn `UserConstructionScript`)