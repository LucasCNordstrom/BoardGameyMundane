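; Card manager actor that runs the deck, hand and on-table cards, and updates WBP_GUI as they change.
; New hands reset and shuffle CurrentDeck from FullDeck, while NextTurn draws from the remaining deck and costs player HP; both respawn BP_Card actors in a row.
; It also spawns two random BP_ChooseCard options, then clears them and has BP_TaskManager choose a new task, repeating the pick when AdditionalCards is set.
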(event `self.ReceiveBeginPlay`
  ;[1 1 1] Begin Play
  (`KismetSystemLibrary.Delay` 0.2)
  (`|ExecutionSequence`
    (:`then_0`
      (set `self.CurrentDeck` (`self.FullDeck`))
      (`KismetSystemLibrary.Delay` 0.2)
      (`self.Event ShuffleDeck`))
    (:`then_1`
      (bind _foundwidgets (`WidgetBlueprintLibrary.GetAllWidgetsOfClass` "/Game/Blueprints/WBP_GUI.WBP_GUI_C"))
      (set `self.GUI` (`|GetArrayItem` _foundwidgets))
      (bind _outactors (`GameplayStatics.GetAllActorsOfClass` "/Game/Blueprints/BP_TaskManager.BP_TaskManager_C"))
      (set `self.TaskManager` (`|GetArrayItem` _outactors))
      (`KismetSystemLibrary.Delay` 0.2)
      (`/Game/Blueprints/WBP_GUI.Event UpdateGUI` (`self.GUI`)))))

(event `Event ChooseCardDone`
  ;[1 1 1] Choose card between tasks
  (for _array_element (`self.CardsToChoose`)
    (`self.K2_DestroyActor` _array_element))
  (`KismetSystemLibrary.Delay` 0.2)
  (`KismetArrayLibrary.Array_Clear` (`self.CardsToChoose`))
  (bind _returnvalue (`GameplayStatics.GetActorOfClass` "/Game/Blueprints/BP_TaskManager.BP_TaskManager_C"))
  (if (`/Game/Blueprints/BP_TaskManager.AdditionalCards` _returnvalue)
    (`self.Event ChooseCard`)
    (set `/Game/Blueprints/BP_TaskManager.AdditionalCards` false _returnvalue))
  (`/Game/Blueprints/BP_TaskManager.Event ChooseNewTask` (`self.TaskManager`)))

(event `Event NewHandOfCards`
  ;[1 1 1] Draw new hand
  (`self.Event ShuffleDeck`)
  (for _index (range (`self.DrawCards`))
    (`KismetArrayLibrary.Array_Set` (`self.CardsInHand`) _index (`|GetArrayItem` (`self.CurrentDeck`)) true)
    (`KismetArrayLibrary.Array_Remove` (`self.CurrentDeck`)))
  (`/Game/Blueprints/WBP_GUI.Event UpdateCurrentDeckGUI` (`self.GUI`))
  (`self.Event SpawnCards`))

(event `Event ChooseCard`
  ;[1 1 1] Choose card between tasks
  (`KismetArrayLibrary.Array_Clear` (`self.CardsToChoose`))
  (for _index (range 1 3)
    (bind _returnvalue (`|SpawnActorFromClass` "/Game/Blueprints/BP_ChooseCard.BP_ChooseCard_C" (`KismetMathLibrary.MakeTransform` (`KismetMathLibrary.MakeVector` 300.0 (+ (`KismetMathLibrary.Conv_IntToDouble` (* _index 450)) (.y (.location (`self.GetTransform`)))))) "AlwaysSpawn" "OverrideRootScale" null (cast `/Game/E_CardTypes` (`KismetMathLibrary.Conv_IntToByte` (`KismetMathLibrary.RandomIntegerInRange` 0 (- (enumcount `/Game/E_CardTypes`) 1)))) null)) ; Spawn a  block
    (`KismetArrayLibrary.Array_Add` (`self.CardsToChoose`) _returnvalue)))

(event `Event AddCardTohand`
  (params (CardToAdd :type "/Game/E_CardTypes Enum" :default "NewEnumerator0"))
  ;[1 1 1] Add Card to Hand
  (`KismetArrayLibrary.Array_Set` (`self.CardsInHand`) (`KismetArrayLibrary.Array_Length` (`self.CardsInHand`)) CardToAdd true))

(event `Event RemoveCardFromHand`
  (params (CardIndex :type Integer))
  ;[1 1 1] Remove Card from hand
  (`KismetArrayLibrary.Array_Remove` (`self.CardsInHand`) CardIndex))

(event `Event AddCardToDeck`
  (params (CardToAdd :type "/Game/E_CardTypes Enum" :default "NewEnumerator0"))
  (bind _currentdeck (`self.CurrentDeck`))
  ;[1 1 1] Add Cards to Deck
  (`KismetArrayLibrary.Array_Set` _currentdeck (`KismetArrayLibrary.Array_Length` _currentdeck) CardToAdd true))

(event `Event RemoveCardFromDeck`
  (params (CardToRemove :type "/Game/E_CardTypes Enum" :default "NewEnumerator0"))
  (bind _currentdeck (`self.CurrentDeck`))
  ;[1 1 1] Remove Cards from Deck
  (`KismetArrayLibrary.Array_Remove` _currentdeck (`KismetArrayLibrary.Array_Find` _currentdeck CardToRemove)))

(event `Event SpawnCards`
  (bind _returnvalue (`self.GetTransform`))
  ;[1 1 1] Spawn Cards in Hand to Board
  (for _array_element (`self.CardsOnTable`)
    (`self.K2_DestroyActor` _array_element))
  (`KismetSystemLibrary.Delay` 0.2)
  (`KismetArrayLibrary.Array_Clear` (`self.CardsOnTable`))
  (for _index (range (`KismetArrayLibrary.Array_Length` (`self.CardsInHand`)))
    (bind _returnvalue_2 (`|SpawnActorFromClass` "/Game/Blueprints/BP_Card.BP_Card_C" (`KismetMathLibrary.MakeTransform` (`KismetMathLibrary.MakeVector` (.x (.location _returnvalue)) (+ (`KismetMathLibrary.Conv_IntToDouble` (* _index 250)) (.y (.location _returnvalue))))) "AlwaysSpawn" "OverrideRootScale" null (`|GetArrayItem` (`self.CardsInHand`) _index) _index null)) ; Spawn a  block
    (`KismetArrayLibrary.Array_Add` (`self.CardsOnTable`) _returnvalue_2)))

(event `Event AddCardToFullDeck`
  (params (CardToAdd :type "/Game/E_CardTypes Enum" :default "NewEnumerator0"))
  (bind _fulldeck (`self.FullDeck`))
  ;[1 1 1] Add Card to FullDeck
  (`KismetArrayLibrary.Array_Set` _fulldeck (`KismetArrayLibrary.Array_Length` _fulldeck) CardToAdd true)
  (`/Game/Blueprints/WBP_GUI.Event AddCardToFullDeck` (`self.GUI`) CardToAdd))

(event `Event ShuffleDeck`
  ;[1 1 1] Reset and Shuffle
  (set `self.CurrentDeck` (`self.FullDeck`))
  (`KismetArrayLibrary.Array_Shuffle` (`self.CurrentDeck`)))

(event `Event RemoveCardsOnTable`
  ;[1 1 1] Remove cards on table
  (for _array_element (`self.CardsOnTable`)
    (`self.K2_DestroyActor` _array_element))
  (`KismetSystemLibrary.Delay` 0.2)
  (`KismetArrayLibrary.Array_Clear` (`self.CardsOnTable`)))

(event `Event NextTurn`
  (bind _gui (`self.GUI`))
  ;[1 1 1] Next Turn
  (`KismetArrayLibrary.Array_Clear` (`self.CardsInHand`))
  (for _index (range 3)
    (bind _output (`|GetArrayItem` (`self.CurrentDeck`) _index))
    (`self.Event AddCardTohand` _output)
    (`self.Event RemoveCardFromDeck` _output))
  (set `self.PlayerHP` (- (`self.PlayerHP`) 1))
  (`/Game/Blueprints/WBP_GUI.Event UpdateGUI` _gui)
  (`/Game/Blueprints/WBP_GUI.Event UpdateCurrentDeckGUI` _gui)
  (`self.Event SpawnCards`))

(fn `UserConstructionScript`)