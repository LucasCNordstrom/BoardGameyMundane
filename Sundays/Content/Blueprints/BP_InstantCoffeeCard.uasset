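; BP_InstantCoffeeCard is a one-shot card effect actor that draws three cards and adds a new card to the deck.
; On BeginPlay it moves cards from the front of BP_CardManager's current deck to the hand, refreshes WBP_GUI and triggers card spawning.
; It then appends one enum-identified card to both the current and full decks, updates the deck display and destroys itself.
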(event `self.ReceiveBeginPlay`
  (bind _currentdeck (`/Game/Blueprints/BP_CardManager.CurrentDeck` (`self.Ref_CardManager`)))
  (bind _output (`|GetArrayItem` _currentdeck))
  ;[1 1 1] Draw 3 cards and add a new card to deck
  (bind _returnvalue (`GameplayStatics.GetActorOfClass` "/Game/Blueprints/BP_CardManager.BP_CardManager_C"))
  (set `self.Ref_CardManager` _returnvalue)
  (for _ (range 4)
    (`/Game/Blueprints/BP_CardManager.Event AddCardTohand` (`self.Ref_CardManager`) _output)
    (`/Game/Blueprints/BP_CardManager.Event RemoveCardFromDeck` (`self.Ref_CardManager`) _output))
  (bind _foundwidgets (`WidgetBlueprintLibrary.GetAllWidgetsOfClass` "/Game/Blueprints/WBP_GUI.WBP_GUI_C"))
  (bind _output_2 (`|GetArrayItem` _foundwidgets))
  (`/Game/Blueprints/WBP_GUI.Event UpdateGUI` _output_2)
  (`/Game/Blueprints/BP_CardManager.Event SpawnCards` (`self.Ref_CardManager`))
  (`KismetArrayLibrary.Array_Add` _currentdeck "NewEnumerator2")
  (`KismetArrayLibrary.Array_Add` (`/Game/Blueprints/BP_CardManager.FullDeck` (`self.Ref_CardManager`)) "NewEnumerator2")
  (`/Game/Blueprints/WBP_GUI.Event UpdateCurrentDeckGUI` _output_2)
  (`self.K2_DestroyActor`))

(fn `UserConstructionScript`)